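; Destruction system component that tracks health for its owning actor and signals when it takes damage or dies.
; On BeginPlay it binds to the owner's OnTakeAnyDamage and routes hits into Damagetaken, which subtracts Maxhealth, not the damage amount, from Currenthealth while alive.
; It then sends the owner a death or damage-taken message and calls the matching Ondeath or Ondamagetaken dispatcher.
; IsAlive reports whether Currenthealth is above zero.
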(event `self.ReceiveBeginPlay`
  (add `Actor.OnTakeAnyDamage` (`self.GetOwner`) (delegate `OnTakeAnyDamage_Event_0`)))

(event `OnTakeAnyDamage_Event_0`
  (params (DamagedActor :type "Actor Object Reference") (Damage :type "Float (single-precision)") (DamageType :type "DamageType Object Reference") (InstigatedBy :type "Controller Object Reference") (DamageCauser :type "Actor Object Reference"))
  (`self.damagetaken` Damage DamageType DamageCauser))

(fn `damagetaken`
  (params (DamageAmount :type "Float (double-precision)") (DamageType :type "DamageType Object Reference") (DamageCause :type "Actor Object Reference"))
  (bind _returnvalue (`self.GetOwner`))
  (if (> (`self.currenthealth`) 0.0)
    (bind _output_get (set `self.currenthealth` (- (`self.currenthealth`) (`self.maxhealth`))))
    (if (<= _output_get 0.0)
      (message `/Game/blueprints/destruction_system/BPI_Damagable.Death` _returnvalue)
      (`self.Ondeath`)
      (else
        (message `/Game/blueprints/destruction_system/BPI_Damagable.Damagetaken` _returnvalue (`local.DamageAmount`) (`local.DamageType`) (`local.DamageCause`))
        (`self.ondamagetaken`)))))

(fn `IsAlive`
  (returns (Alive :type Boolean))
  (return (> (`self.currenthealth`) 0.0)))