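; Door Blueprint that swings a pair of doors open when its Usedoor event fires.
; Usedoor calls opendoor, which restarts two timelines in sequence, one per leaf.
; Each timeline lerps its door's relative yaw from closed to open angle and sets the Opendoor flag on every update.
; The graph only opens the doors; it has no closing logic and never checks the flag.
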(event `opendoor`
  (`|ExecutionSequence`
    (:`then_0`
      (bind (_direction _opendoor) (`Timeline|opendoor2` :!via `PlayFromStart`)
        (:`Update`
          (`SceneComponent.K2_SetRelativeRotation` (`self.leftdoor`) (`KismetMathLibrary.MakeRotator` 0.0 0.0 (`KismetMathLibrary.Lerp` (`self.leftdoorclosed`) (`self.leftdooropen`) _opendoor)) false false)
          (set `self.opendoor?` true))))
    (:`then_1`
      (bind (_direction_2 _opendoor_2) (`Timeline|Timeline` :!via `PlayFromStart`)
        (:`Update`
          (`SceneComponent.K2_SetRelativeRotation` (`self.rightdoor`) (`KismetMathLibrary.MakeRotator` 0.0 0.0 (`KismetMathLibrary.Lerp` (`self.rightdoorclose`) (`self.rightdooropen`) _opendoor_2)) false false)
          (set `self.opendoor?` true))))))

(event `/Game/interfaces/usedoorinterface.usedoor`
  (`self.opendoor`))

(fn `UserConstructionScript`)