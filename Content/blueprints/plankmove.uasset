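; Rotating plank actor that swings a static mesh between closed and opened roll angles.
; The Beamuse event plays a timeline from the start to lerp the roll, setting Openbeam on each update, while overlapping Boxcollision1 plays it in reverse from the end.
; Entering or leaving Boxcollision toggles Timereversable on the overlapping BP_ThirdPersonCharacter.
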(event `/Game/interfaces/beaminterface.beamuse`
  (`self.movebeam`))

(event `movebeam`
  (bind (_direction _newtrack_0) (`Timeline|Timeline` :!via `PlayFromStart` :!label _label)
    (:`Update`
      (`SceneComponent.K2_SetRelativeRotation` (`self.StaticMesh`) (`KismetMathLibrary.MakeRotator` (`KismetMathLibrary.Lerp` (`self.beamcloses`) (`self.beamopened`) _newtrack_0)) false false)
      (set `self.openbeam` true))))

(event `self. boxcollision1.OnComponentBeginOverlap`
  (params (OverlappedComponent :type "PrimitiveComponent Object Reference") (OtherActor :type "Actor Object Reference") (OtherComp :type "PrimitiveComponent Object Reference") (OtherBodyIndex :type Integer) (bFromSweep :type Boolean) (SweepResult :type "HitResult Structure (by ref)"))
  (goto _label :!via `ReverseFromEnd`))

(event `self. boxcollision.OnComponentBeginOverlap`
  (params (OverlappedComponent :type "PrimitiveComponent Object Reference") (OtherActor :type "Actor Object Reference") (OtherComp :type "PrimitiveComponent Object Reference") (OtherBodyIndex :type Integer) (bFromSweep :type Boolean) (SweepResult :type "HitResult Structure (by ref)"))
  (bind _asbp_third_person_character (cast `/Game/ThirdPerson/Blueprints/BP_ThirdPersonCharacter` OtherActor))
  (set `/Game/ThirdPerson/Blueprints/BP_ThirdPersonCharacter.timereversable?` true _asbp_third_person_character)
  (set `self.Mesh` (`Character.Mesh` _asbp_third_person_character)))

(event `self. boxcollision.OnComponentEndOverlap`
  (params (OverlappedComponent :type "PrimitiveComponent Object Reference") (OtherActor :type "Actor Object Reference") (OtherComp :type "PrimitiveComponent Object Reference") (OtherBodyIndex :type Integer))
  (bind _asbp_third_person_character (cast `/Game/ThirdPerson/Blueprints/BP_ThirdPersonCharacter` OtherActor))
  (set `/Game/ThirdPerson/Blueprints/BP_ThirdPersonCharacter.timereversable?` false _asbp_third_person_character)
  (set `self.Mesh` (`Character.Mesh` _asbp_third_person_character)))

(fn `UserConstructionScript`)